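; BP_Alien is a spider enemy that chases the player character and plays an attack montage at close range.
; A self-restarting AI MoveTo loop drives pursuit, while Tick checks distance and pauses CharacterMovement during the montage.
; Damage reduces health; on death the alien increments the marine's kill count, disables collision, destroys itself and reports to BP_MarsMarine_GameMode.
; The attack applies no damage in this Blueprint.
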(event EventBeginPlay
  ;[1 1 1] movement
  (AI|AIMoveTo self "0, 0, 0" (Game|GetPlayerCharacter 0) 5.0 false :!label _label
    (:OnSuccess
      _)
    (:OnFail
      _))
  (if (not (Variables|Default|Getis%20dead))
    (goto _label)))

(event EventTick
  (params (DeltaSeconds :type Float%20%28single-precision%29))
  (bind _charactermovement (Variables|Character|GetCharacterMovement))
  ;[1 1 1] attack
  (if (not (Variables|Default|Getis%20dead))
    (if (CallFunction|IsinAttackRange)
      (if (not (CallFunction|IsAttacking))
        (Components|Activation|Deactivate _charactermovement)
        (Animation|Montage|PlayMontage (Variables|Character|GetMesh) "/Game/Characters/Enemy_Great_Spider/Animations/spider_attack.spider_attack"
          (:OnCompleted
            (Components|Activation|Activate _charactermovement false)))))))

(event Game|Damage|EventAnyDamage
  (params (Damage :type Float%20%28single-precision%29) (DamageType :type Damage%20Type%20Object%20Reference) (InstigatedBy :type Controller%20Object%20Reference) (DamageCauser :type Actor%20Object%20Reference))
  ;[1 1 1] damage system
  (CallFunction|Death Damage)
  (if (Variables|Default|Getis%20dead)
    (Components|Activation|Deactivate (Variables|Character|GetCharacterMovement))
    (CallFunction|AddKill)
    (Collision|SetCollisionEnabled (Variables|Collision|GetCapsuleComponent) "NoCollision")
    (Actor|DestroyActor)
    (bind _asbp_mars_marine_game_mode (Utilities|Casting|CastToBP_MarsMarine_GameMode (Game|GetGameMode)))
    (Default|RegisterSpiderDeath _asbp_mars_marine_game_mode self)))

(fn ConstructionScript)

(fn IsinAttackRange
  (return (< (Transformation|GetDistanceTo (Game|GetPlayerCharacter 0)) 1e+02)))

(fn IsAttacking
  (return (Animation|Montage|MontageIsPlaying (Components|SkeletalMesh|GetAnimInstance (Variables|Character|GetMesh)) "/Game/Characters/Enemy_Great_Spider/Animations/spider_attack.spider_attack")))

(fn Death
  (params (damage :type Float%20%28single-precision%29))
  (bind _output_get (Variables|Default|Sethealth (- (Variables|Default|Gethealth) damage)))
  (if (<= _output_get 0.0)
    (bind _output_get_2 (Variables|Default|Setis%20dead true))
    (return _output_get_2)))

(fn AddKill
  (bind _asbp_marine (Utilities|Casting|CastToBP_Marine (Game|GetPlayerCharacter 0)))
  (Variables|Default|SetAs%20BP%20Marine _asbp_marine)
  (bind _result (Math|Integer|IncrementInt (Variables|/Game/Blueprints/Pawns/BP_Marine.BP_Marine_C|GetKills (Variables|Default|GetAs%20BP%20Marine)))
    (:%20%20
      (Variables|/Game/Blueprints/Pawns/BP_Marine.BP_Marine_C|SetKills (Variables|Default|GetAs%20BP%20Marine) _result))))